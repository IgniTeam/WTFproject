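; Base enemy character that damages the player, takes damage and rewards the player when killed.
; Attack hits the player character directly with no range check, toggling an Attacking flag behind a DoOnce that resets after a short delay.
; At zero HP, Death runs once: it ragdolls, detaches the controller, notifies GM_Main, spawns the Reward actor and gives BP_Hero one of two weighted-random buffs before destroying itself.
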(event Custom|Death
  (Physics|SetSimulatePhysics (Variables|Character|GetMesh) true)
  (Components|Movement|StopMovementImmediately (Variables|Character|GetCharacterMovement))
  (Class|Pawn|DetachfromControllerPendingDestroy)
  (bind _asgm_main (Utilities|Casting|CastToGM_Main (Game|GetGameMode)))
  (Default|RemoveEnemy _asgm_main)
  (Game|SpawnActorfromClass (Variables|Default|GetReward) (Transformation|GetActorTransform) "AlwaysSpawn" 0 0)
  (bind _asbp_hero (Utilities|Casting|CastToBP_Hero (Game|GetPlayerCharacter 0)))
  (if (Math|Random|RandomBoolwithWeight 0.25)
    (Variables|Default|SetBaff "NewEnumerator0")
    (else
      (Variables|Default|SetBaff "NewEnumerator2")))
  (Default|BuffHero _asbp_hero (Variables|Default|GetBaff))
  (Utilities|FlowControl|Delay 1.0)
  (Actor|DestroyActor))

(event EventBeginPlay)

(event EventAttack
  (Utilities|FlowControl|DoOnce false :!label _label
    (:Completed
      (Game|Damage|ApplyDamage (Game|GetPlayerCharacter 0) (Variables|Default|GetDamage) 0 self)
      (Variables|Default|SetAttacking true)
      (Audio|PlaySound2D "/Game/Proj/Sounds/426308__mtjohnson__hollywood-punch.426308__mtjohnson__hollywood-punch" 1.0 1.0 0.0 0 0)
      (Utilities|FlowControl|Delay 0.5)
      (Variables|Default|SetAttacking false)
      (Development|PrintString "Hello")
      (goto _label Reset))))

(event Game|Damage|EventAnyDamage
  (params (Damage :type Float%20%28single-precision%29) (DamageType :type Damage%20Type%20Object%20Reference) (InstigatedBy :type Controller%20Object%20Reference) (DamageCauser :type Actor%20Object%20Reference))
  (Variables|Default|SetHP (- (Variables|Default|GetHP) Damage))
  (if (<= (Variables|Default|GetHP) 0.0)
    (Utilities|FlowControl|DoOnce false
      (:Completed
        (CallFunction|Death)))))

(fn ConstructionScript)