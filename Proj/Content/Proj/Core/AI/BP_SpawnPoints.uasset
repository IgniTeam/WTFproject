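; BP_SpawnPoints is an enemy spawn point that creates a random enemy at its location when play begins.
; It shuffles its Enemies array and spawns the first class slightly above itself.
; GM_Main's BossCounter selects which document-style or other item may become the enemy's Reward through weighted rolls, chained at one stage, with none at the earliest stages.
; It then calls AddEnemy on the game mode to register the spawn.
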(event EventBeginPlay
  (bind _returnvalue (Transformation|GetActorTransform))
  (bind _returnvalue_2 (Math|Random|RandomBoolwithWeight 0.25))
  (bind _enemies (Variables|Default|GetEnemies))
  (Utilities|Array|Shuffle _enemies)
  (bind _returnvalue_3 (Game|SpawnActorfromClass (Utilities|Array|Get(acopy) _enemies) (Math|Transform|MakeTransform (Math|Vector|MakeVector (.x (.location _returnvalue)) (.y (.location _returnvalue)) (+ (.z (.location _returnvalue)) 2e+01)) (.rotation _returnvalue) (.scale _returnvalue)) "AdjustIfPossibleButAlwaysSpawn" 0 0))
  (bind _asgm_main (Utilities|Casting|CastToGM_Main (Game|GetGameMode)))
  (switch int (Variables|/Game/Proj/Core/GM_Main.GM_Main_C|GetBossCounter _asgm_main)
    (:Default
      (if (Math|Random|RandomBoolwithWeight 0.25) :!label _label
        (Variables|/Game/Proj/Core/AI/BP_EnemyBase.BP_EnemyBase_C|SetReward _returnvalue_3 "/Game/Proj/Placeables/Interactables/Documents/BP_2NDFL.BP_2NDFL_C")))
    (:0
      _)
    (:1
      _)
    (:2
      (goto _label))
    (:3
      (if (Math|Random|RandomBoolwithWeight 0.25)
        (Variables|/Game/Proj/Core/AI/BP_EnemyBase.BP_EnemyBase_C|SetReward _returnvalue_3 "/Game/Proj/Placeables/Interactables/Documents/BP_Passport.BP_Passport_C")))
    (:4
      (if (Math|Random|RandomBoolwithWeight 0.25)
        (Variables|/Game/Proj/Core/AI/BP_EnemyBase.BP_EnemyBase_C|SetReward _returnvalue_3 "/Game/Proj/Placeables/Interactables/Documents/BP_Birth.BP_Birth_C")
        (elif _returnvalue_2
          (Variables|/Game/Proj/Core/AI/BP_EnemyBase.BP_EnemyBase_C|SetReward _returnvalue_3 "/Game/Proj/Placeables/Interactables/Documents/BP_Bank.BP_Bank_C")
          (elif _returnvalue_2
            (Variables|/Game/Proj/Core/AI/BP_EnemyBase.BP_EnemyBase_C|SetReward _returnvalue_3 "/Game/Proj/Placeables/Interactables/Documents/BP_Drug.BP_Drug_C")
            (elif _returnvalue_2
              (Variables|/Game/Proj/Core/AI/BP_EnemyBase.BP_EnemyBase_C|SetReward _returnvalue_3 "/Game/Proj/Placeables/Interactables/Documents/BP_DriverCard.BP_DriverCard_C")))))))
  (bind _asgm_main_2 (Utilities|Casting|CastToGM_Main (Game|GetGameMode)))
  (Default|AddEnemy _asgm_main_2))

(fn ConstructionScript)