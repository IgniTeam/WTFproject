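; GM_Main is the game mode Blueprint that runs streamed-level progression and tracks living enemies.
; LoadLevel shows a loading widget, unloads the previous level, destroys enemies, streams in a named or random level and moves the player to a PlayerStart.
; Random picks come from a shuffled pool without repeats, refilled from the master list when empty.
; Each enemy removal increments the hero's SuperShot, and clearing all enemies calls LiftDown on the elevator.
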(event Custom|LoadLevel
  (params (LevelToLoad :type Name))
  (bind _currentlevels (Variables|Default|GetCurrentLevels))
  (bind _output (Utilities|Array|Get(acopy) _currentlevels))
  (Utilities|IsValid (Variables|Default|GetLoadingWidget)
    (:Is%20Valid
      (if (UserInterface|Viewport|IsinViewport (Variables|Default|GetLoadingWidget))
        (Widget|RemovefromParent (Variables|Default|GetLoadingWidget))
        (else
          (bind _returnvalue (UserInterface|CreateWidget "/Game/Proj/Core/UI/WB_Loading.WB_Loading_C" :!label _label))
          (Variables|Default|SetLoadingWidget _returnvalue)
          (UserInterface|Viewport|AddtoViewport _returnvalue 0))))
    (:Is%20Not%20Valid
      (goto _label)))
  (Game|UnloadStreamLevel(byName) (Variables|Default|GetPreviousLevel) false)
  (bind _outactors (Actor|GetAllActorsOfClass "/Game/Proj/Core/AI/BP_EnemyBase.BP_EnemyBase_C"))
  (for _array_element _outactors
    (Actor|DestroyActor _array_element))
  (Variables|Default|SetEnemiesCount 0)
  (if (Utilities|Name|Equal(Name) LevelToLoad "None")
    (Utilities|Array|Shuffle _currentlevels)
    (Variables|Default|SetPreviousLevel _output)
    (Game|LoadStreamLevel(byName) _output true)
    (Utilities|Array|RemoveItem _currentlevels _output)
    (else
      (Game|LoadStreamLevel(byName) LevelToLoad true)
      (Variables|Default|SetPreviousLevel LevelToLoad)))
  (bind _outactors_2 (Actor|GetAllActorsOfClass "/Script/Engine.PlayerStart"))
  (Transformation|SetActorLocation (Game|GetPlayerCharacter 0) (Transformation|GetActorLocation (Utilities|Array|Get(acopy) _outactors_2)) false false)
  (Utilities|FlowControl|Delay 3.0)
  (Widget|RemovefromParent _returnvalue)
  (if (== (Utilities|Array|Length (Variables|Default|GetCurrentLevels)) 0)
    (CallFunction|ReloadLevels)))

(event Custom|RemoveEnemy
  (bind _character (Variables|Default|GetCharacter))
  (bind _output_get (Variables|Default|SetEnemiesCount (- (Variables|Default|GetEnemiesCount) 1)))
  (Development|PrintString (Utilities|String|ToString(Integer) _output_get))
  (Variables|/Game/Proj/Core/BP_Hero.BP_Hero_C|SetSuperShot _character (+ (Variables|/Game/Proj/Core/BP_Hero.BP_Hero_C|GetSuperShot _character) 1.0))
  (if (<= _output_get 0)
    (bind _outactors (Actor|GetAllActorsOfClass "/Game/Proj/Placeables/Interactables/Elevator/BP_Elevator.BP_Elevator_C"))
    (Default|LiftDown (Utilities|Array|Get(acopy) _outactors))
    (Development|PrintString "Removed")))

(event Custom|AddEnemy
  (bind _output_get (Variables|Default|SetEnemiesCount (+ (Variables|Default|GetEnemiesCount) 1)))
  (Development|PrintString (Utilities|String|ToString(Integer) _output_get)))

(event Custom|ReloadLevels
  (Utilities|Array|Clear (Variables|Default|GetCurrentLevels))
  (Variables|Default|SetCurrentLevels (Variables|Default|GetLevels)))

(event EventBeginPlay
  (CallFunction|ReloadLevels)
  (bind _asbp_hero (Utilities|Casting|CastToBP_Hero (Game|GetPlayerCharacter 0)))
  (Variables|Default|SetCharacter _asbp_hero))

(fn ConstructionScript)