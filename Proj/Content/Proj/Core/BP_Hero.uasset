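; Player hero for a shooter with world-axis movement, separate-axis aiming and wheel zoom.
; Left click fires two damaging line traces with recoil impulse and effects, gated by a DoOnce cooldown.
; A charged SuperShot on E temporarily enables timer-driven automatic fire that bypasses the gate.
; Also handles HP, timed speed and healing buffs, HUD and inventory updates, a menu whose toggle always sets pause true, and death loading Transit.
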(event Custom|Death
  (Input|DisableInput (Game|GetPlayerController 0))
  (bind _returnvalue (UserInterface|CreateWidget "/Game/Proj/Core/UI/WB_Loading.WB_Loading_C"))
  (UserInterface|Viewport|AddtoViewport _returnvalue 0)
  (Game|OpenLevel(byName) "Transit"))

(event Custom|UpdateFoundItems
  (Default|UpdateInventoryUI (Variables|/Game/Proj/Core/UI/WB_Main.WB_Main_C|GetWB_Inventory (Variables|Default|GetWBMain)) (Variables|Default|GetSDoc)))

(event Custom|BuffHero
  (params (Baff :type EBaffs%20Enum :default "NewEnumerator0"))
  (bind _charactermovement (Variables|Character|GetCharacterMovement))
  (bind _wbmain (Variables|Default|GetWBMain))
  (switch Utilities|FlowControl|Switch|SwitchonEBaffs Baff
    (:NewEnumerator0
      (Variables|/Script/Engine.CharacterMovementComponent|SetMaxWalkSpeed _charactermovement (Variables|Default|GetRunSpeed))
      (Default|Buff _wbmain "Скорость увеличена!")
      (Utilities|FlowControl|RetriggerableDelay 1e+01)
      (Variables|/Script/Engine.CharacterMovementComponent|SetMaxWalkSpeed _charactermovement (Variables|Default|GetWalkSpeed)))
    (:NewEnumerator2
      (Variables|Default|SetHP (Math|Float|Clamp(Float) (+ (Variables|Default|GetHP) 1e+01) 0.0 1e+02))
      (Default|Buff _wbmain "Здоровье увеличено!"))))

(event Custom|Fire
  (bind _linetrace1 (Variables|Default|GetLinetrace1))
  (bind _linetrace2 (Variables|Default|GetLinetrace2))
  (bind _returnvalue (Transformation|GetWorldLocation _linetrace2))
  (bind _returnvalue_2 (Transformation|GetWorldLocation _linetrace1))
  (Utilities|FlowControl|Sequence
    (:then_0
      (bind (_outhit _returnvalue_3) (Collision|LineTraceByChannel _returnvalue_2 (+ _returnvalue_2 (* (Math|Vector|GetForwardVector (Variables|Collision|GetCapsuleComponent)) 1.5e+03)) "TraceTypeQuery1" false 0 "ForDuration"))
      (if _returnvalue_3
        (Game|Damage|ApplyDamage (.HitActor (Collision|BreakHitResult _outhit)) 1e+01 0 self))
      (Effects|SpawnEmitteratLocation "/Game/InfinityBladeEffects/Effects/FX_Monsters/FX_Monster_Gruntling/Master/P_BackPack_MuzzleFlash.P_BackPack_MuzzleFlash" (.Location (Collision|BreakHitResult _outhit)) "0, 0, 0" "0.500000,0.500000,0.500000"))
    (:then_1
      (bind (_outhit_2 _returnvalue_4) (Collision|LineTraceByChannel _returnvalue (+ _returnvalue (* (Math|Vector|GetForwardVector (Variables|Collision|GetCapsuleComponent)) 1.5e+03)) "TraceTypeQuery1" false 0 "ForDuration"))
      (if _returnvalue_4
        (Game|Damage|ApplyDamage (.HitActor (Collision|BreakHitResult _outhit_2)) 1e+01 0 self))
      (Effects|SpawnEmitteratLocation "/Game/InfinityBladeEffects/Effects/FX_Monsters/FX_Monster_Gruntling/Master/P_BackPack_MuzzleFlash.P_BackPack_MuzzleFlash" (.Location (Collision|BreakHitResult _outhit_2)) "0, 0, 0" "0.500000,0.500000,0.500000")))
  (Physics|AddImpulse (Variables|Character|GetCharacterMovement) (* (Math|Vector|GetForwardVector (Variables|Collision|GetCapsuleComponent)) -1e+03) true)
  (Effects|SpawnEmitteratLocation "/Game/InfinityBladeEffects/Effects/FX_Monsters/FX_Monster_Gruntling/Master/P_BackPack_MuzzleFlash.P_BackPack_MuzzleFlash" (Transformation|GetSocketLocation (Variables|Default|GetSkeletalMesh) "Muzzle") "0, 0, 0" "0.200000,0.200000,0.200000")
  (Audio|PlaySound2D "/Game/Proj/Sounds/51464__smcameron__bombexplosion.51464__smcameron__bombexplosion" 1.0 1.0 0.0 0 0)
  (Utilities|FlowControl|RetriggerableDelay 0.5)
  (Utilities|FlowControl|DoOnce false) ; enters at Reset
)

(event EventBeginPlay
  (bind _returnvalue (UserInterface|CreateWidget "/Game/Proj/Core/UI/WB_Main.WB_Main_C"))
  (UserInterface|Viewport|AddtoViewport _returnvalue 0)
  (Variables|Default|SetWBMain _returnvalue))

(event Game|Damage|EventAnyDamage
  (params (Damage :type Float%20%28single-precision%29) (DamageType :type Damage%20Type%20Object%20Reference) (InstigatedBy :type Controller%20Object%20Reference) (DamageCauser :type Actor%20Object%20Reference))
  (bind _output_get (Variables|Default|SetHP (- (Variables|Default|GetHP) Damage)))
  (Development|PrintString (Utilities|String|ToString(Float) _output_get) true true "(R=1.000000,G=0.695082,B=0.000000,A=1.000000)")
  (if (<= _output_get 0.0)
    (CallFunction|Death)))

(event Input|AxisEvents|InputAxisMoveForward
  (params (AxisValue :type Float%20%28single-precision%29))
  (Pawn|Input|AddMovementInput "1.000000, 0, 0" AxisValue false))

(event Input|AxisEvents|InputAxisMoveRight
  (params (AxisValue :type Float%20%28single-precision%29))
  (Pawn|Input|AddMovementInput "0,1.000000, 0" AxisValue false))

(event Input|AxisEvents|InputAxisTurn
  (params (AxisValue :type Float%20%28single-precision%29))
  (if (!= AxisValue 0.0)
    (Transformation|SetWorldRotation (Variables|Character|GetMesh) (Math|Conversions|RotationFromXVector (Math|Vector|MakeVector (Input|AxisValues|GetTurn) (* (Input|AxisValues|GetTurnForward) -1.0) 0.0)) false false)))

(event Input|AxisEvents|InputAxisTurnForward
  (params (AxisValue :type Float%20%28single-precision%29))
  (if (!= AxisValue 0.0)
    (Transformation|SetWorldRotation (Variables|Character|GetMesh) (Math|Conversions|RotationFromXVector (Math|Vector|MakeVector (Input|AxisValues|GetTurn) (* (Input|AxisValues|GetTurnForward) -1.0) 0.0)) false false)))

(event Input|KeyboardEvents|E
  (params (Key :type Key%20Structure :default "None")))

(event Input|MouseEvents|LeftMouseButton
  (params (Key :type Key%20Structure :default "None"))
  (bind _linetrace1 (Variables|Default|GetLinetrace1))
  (bind _linetrace2 (Variables|Default|GetLinetrace2))
  (bind _returnvalue (Transformation|GetWorldLocation _linetrace2))
  (bind _returnvalue_2 (Transformation|GetWorldLocation _linetrace1))
  (:Pressed
    (if (Variables|Default|GetAutomaticFire)
      (bind _returnvalue_3 (Utilities|Time|SetTimerbyEvent (delegate Custom|Fire) 0.2 true))
      (else
        (Utilities|FlowControl|DoOnce false :!label _label
          (:Completed
            (Utilities|FlowControl|Sequence
              (:then_0
                (bind (_outhit _returnvalue_4) (Collision|LineTraceByChannel _returnvalue_2 (+ _returnvalue_2 (* (Math|Vector|GetForwardVector (Variables|Collision|GetCapsuleComponent)) 1.5e+03)) "TraceTypeQuery1" false 0 "ForDuration"))
                (if _returnvalue_4
                  (Game|Damage|ApplyDamage (.HitActor (Collision|BreakHitResult _outhit)) 1e+01 0 self))
                (Effects|SpawnEmitteratLocation "/Game/InfinityBladeEffects/Effects/FX_Monsters/FX_Monster_Gruntling/Master/P_BackPack_MuzzleFlash.P_BackPack_MuzzleFlash" (.Location (Collision|BreakHitResult _outhit)) "0, 0, 0" "0.500000,0.500000,0.500000"))
              (:then_1
                (bind (_outhit_2 _returnvalue_5) (Collision|LineTraceByChannel _returnvalue (+ _returnvalue (* (Math|Vector|GetForwardVector (Variables|Collision|GetCapsuleComponent)) 1.5e+03)) "TraceTypeQuery1" false 0 "ForDuration"))
                (if _returnvalue_5
                  (Game|Damage|ApplyDamage (.HitActor (Collision|BreakHitResult _outhit_2)) 1e+01 0 self))
                (Effects|SpawnEmitteratLocation "/Game/InfinityBladeEffects/Effects/FX_Monsters/FX_Monster_Gruntling/Master/P_BackPack_MuzzleFlash.P_BackPack_MuzzleFlash" (.Location (Collision|BreakHitResult _outhit_2)) "0, 0, 0" "0.500000,0.500000,0.500000")))
            (Physics|AddImpulse (Variables|Character|GetCharacterMovement) (* (Math|Vector|GetForwardVector (Variables|Collision|GetCapsuleComponent)) -1e+03) true)
            (Effects|SpawnEmitteratLocation "/Game/InfinityBladeEffects/Effects/FX_Monsters/FX_Monster_Gruntling/Master/P_BackPack_MuzzleFlash.P_BackPack_MuzzleFlash" (Transformation|GetSocketLocation (Variables|Default|GetSkeletalMesh) "Muzzle") "0, 0, 0" "0.200000,0.200000,0.200000")
            (Audio|PlaySound2D "/Game/Proj/Sounds/51464__smcameron__bombexplosion.51464__smcameron__bombexplosion" 1.0 1.0 0.0 0 0)
            (Utilities|FlowControl|RetriggerableDelay 0.5)
            (goto _label Reset))))))
  (:Released
    (Utilities|Time|ClearandInvalidateTimerbyHandle _returnvalue_3)))

(event Input|MouseEvents|MouseWheelDown
  (params (Key :type Key%20Structure :default "None"))
  (bind _springarm1 (Variables|Default|GetSpringArm1))
  (:Pressed
    (Variables|/Script/Engine.SpringArmComponent|SetTargetArmLength _springarm1 (Math|Float|Clamp(Float) (+ (Variables|/Script/Engine.SpringArmComponent|GetTargetArmLength _springarm1) 5e+01) 8e+02 1.4e+03))))

(event Input|MouseEvents|MouseWheelUp
  (params (Key :type Key%20Structure :default "None"))
  (bind _springarm1 (Variables|Default|GetSpringArm1))
  (:Pressed
    (Variables|/Script/Engine.SpringArmComponent|SetTargetArmLength _springarm1 (Math|Float|Clamp(Float) (- (Variables|/Script/Engine.SpringArmComponent|GetTargetArmLength _springarm1) 5e+01) 8e+02 1.4e+03))))

(event Input|KeyboardEvents|P
  (params (Key :type Key%20Structure :default "None"))
  (:Pressed
    (Utilities|IsValid (Variables|Default|GetInGameMenu)
      (:Is%20Valid
        (if (UserInterface|Viewport|IsinViewport (Variables|Default|GetInGameMenu))
          (Widget|RemovefromParent (Variables|Default|GetInGameMenu))
          (Game|SetGamePaused true)
          (else
            (UserInterface|Viewport|AddtoViewport (Variables|Default|GetInGameMenu) 0 :!label _label)
            (Game|SetGamePaused true))))
      (:Is%20Not%20Valid
        (bind _returnvalue (UserInterface|CreateWidget "/Game/Proj/Core/UI/WB_InGameMenu.WB_InGameMenu_C"))
        (Variables|Default|SetInGameMenu _returnvalue)
        (goto _label)))))

(event Input|KeyboardEvents|Escape
  (params (Key :type Key%20Structure :default "None")))

(event Input|KeyboardEvents|E
  (params (Key :type Key%20Structure :default "None"))
  (:Pressed
    (if (>= (Variables|Default|GetSuperShot) 1e+01)
      (Variables|Default|SetSuperShot 0.0)
      (Variables|Default|SetAutomaticFire true)
      (Utilities|FlowControl|RetriggerableDelay 1e+01)
      (Variables|Default|SetAutomaticFire false)
      (Utilities|Time|ClearandInvalidateTimerbyHandle (stale Input|MouseEvents|LeftMouseButton _returnvalue_3)))))

(fn ConstructionScript)