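; Elevator that acts as a level exit, loading the next level through GM_Main once no enemies remain.
; When the player enters its sphere, it checks their SDoc item classes against GM_Main's NeededItems, removing matches.
; A missing item loads level "None" and optionally increments BossCounter; a complete set reloads levels and loads "boss".
; A box trigger drives the LockDoors timeline sliding two walls, reversed on entry and played on exit.
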(event OnComponentBeginOverlap(Sphere)
  (params (OverlappedComponent :type Primitive%20Component%20Object%20Reference) (OtherActor :type Actor%20Object%20Reference) (OtherComp :type Primitive%20Component%20Object%20Reference) (OtherBodyIndex :type Integer) (bFromSweep :type Boolean) (SweepResult :type Hit%20Result%20Structure%20%28by%20ref%29))
  (if (== OtherActor (Variables|Default|GetCharacter))
    (bind _asgm_main (Utilities|Casting|CastToGM_Main (Game|GetGameMode)))
    (if (<= (Variables|/Game/Proj/Core/GM_Main.GM_Main_C|GetEnemiesCount _asgm_main) 0)
      (for _array_element (Variables|/Game/Proj/Core/BP_Hero.BP_Hero_C|GetSDoc (Variables|Default|GetCharacter))
        (Utilities|Array|Add (Variables|Default|GetTemp) (.class _array_element)))
      (bind _asgm_main_2 (Utilities|Casting|CastToGM_Main (Game|GetGameMode)))
      (bind _array_element_2 (Utilities|Array|ForEachLoopwithBreak (Variables|/Game/Proj/Core/GM_Main.GM_Main_C|GetNeededItems _asgm_main_2) :!label _label)
        (:LoopBody
          (if (== (Utilities|Array|FindItem (Variables|Default|GetTemp) _array_element_2) -1)
            (Utilities|FlowControl|Sequence
              (:then_0
                (Variables|Default|SetHaveNeededItems false)
                (goto _label Break))
              (:then_1
                (Default|LoadLevel _asgm_main_2 "None")
                (if (Variables|Default|GetIncreaseCounter)
                  (bind _asgm_main_3 (Utilities|Casting|CastToGM_Main (Game|GetGameMode)))
                  (Variables|/Game/Proj/Core/GM_Main.GM_Main_C|SetBossCounter _asgm_main_3 (+ (Variables|/Game/Proj/Core/GM_Main.GM_Main_C|GetBossCounter _asgm_main_3) 1)))))
            (else
              (Utilities|Array|RemoveItem (Variables|/Game/Proj/Core/GM_Main.GM_Main_C|GetNeededItems _asgm_main_2) _array_element_2))))
        (:Completed
          (if (== (Utilities|Array|Length (Variables|/Game/Proj/Core/GM_Main.GM_Main_C|GetNeededItems _asgm_main_2)) 0)
            (if (Variables|Default|GetHaveNeededItems)
              (Default|ReloadLevels _asgm_main_2)
              (Default|LoadLevel _asgm_main_2 "boss"))))))))

(event OnComponentEndOverlap(Box)
  (params (OverlappedComponent :type Primitive%20Component%20Object%20Reference) (OtherActor :type Actor%20Object%20Reference) (OtherComp :type Primitive%20Component%20Object%20Reference) (OtherBodyIndex :type Integer))
  (if (== OtherActor (Variables|Default|GetCharacter))
    (bind (_direction _wall1 _wall2) (Timeline|LockDoors Play)
      (:Update
        (Transformation|SetRelativeLocation (Variables|Default|GetWall1) (Math|Vector|MakeVector 0.0 _wall1 0.0) false false)
        (Transformation|SetRelativeLocation (Variables|Default|GetWall2) (Math|Vector|MakeVector 0.0 _wall2 0.0) false false)))))

(event OnComponentBeginOverlap(Box)
  (params (OverlappedComponent :type Primitive%20Component%20Object%20Reference) (OtherActor :type Actor%20Object%20Reference) (OtherComp :type Primitive%20Component%20Object%20Reference) (OtherBodyIndex :type Integer) (bFromSweep :type Boolean) (SweepResult :type Hit%20Result%20Structure%20%28by%20ref%29))
  (if (== OtherActor (Variables|Default|GetCharacter))
    (bind (_direction _wall1 _wall2) (Timeline|LockDoors Reverse)
      (:Update
        (Transformation|SetRelativeLocation (Variables|Default|GetWall1) (Math|Vector|MakeVector 0.0 _wall1 0.0) false false)
        (Transformation|SetRelativeLocation (Variables|Default|GetWall2) (Math|Vector|MakeVector 0.0 _wall2 0.0) false false)))))

(event Custom|LiftDown)

(event EventBeginPlay
  (|CallParentFunction)
  (bind _asbp_hero (Utilities|Casting|CastToBP_Hero (Game|GetPlayerCharacter 0)))
  (Variables|Default|SetCharacter _asbp_hero))

(event Collision|EventActorBeginOverlap
  (params (OtherActor :type Actor%20Object%20Reference))
  (|CallParentFunction OtherActor) ; This node is disabled and will not be called.\nDrag off pins to build functionality.
)

(event EventTick
  (params (DeltaSeconds :type Float%20%28single-precision%29))
  (|CallParentFunction DeltaSeconds) ; This node is disabled and will not be called.\nDrag off pins to build functionality.
)

(fn ConstructionScript
  (|CallParentFunction))