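; Collectible document pickup that the hero gains by walking into its sphere.
; On begin play it fills in its document info struct with its own class, keeping the name and image.
; On overlap with BP_Hero it adds that info uniquely to the hero's document list, refreshes found items, and destroys itself.
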(event OnComponentBeginOverlap(Sphere)
  (params (OverlappedComponent :type Primitive%20Component%20Object%20Reference) (OtherActor :type Actor%20Object%20Reference) (OtherComp :type Primitive%20Component%20Object%20Reference) (OtherBodyIndex :type Integer) (bFromSweep :type Boolean) (SweepResult :type Hit%20Result%20Structure%20%28by%20ref%29))
  (bind _asbp_hero (Utilities|Casting|CastToBP_Hero OtherActor))
  (Utilities|Array|AddUnique (Variables|/Game/Proj/Core/BP_Hero.BP_Hero_C|GetSDoc _asbp_hero) (Variables|Default|GetDocInfo))
  (Default|UpdateFoundItems _asbp_hero)
  (Actor|DestroyActor))

(event EventBeginPlay
  (|CallParentFunction)
  (Variables|Default|SetDocInfo (Utilities|Struct|MakeSDocs (.name (Variables|Default|GetDocInfo)) (.image (Variables|Default|GetDocInfo)) (Utilities|GetClass self))))

(event Collision|EventActorBeginOverlap
  (params (OtherActor :type Actor%20Object%20Reference))
  (|CallParentFunction OtherActor) ; This node is disabled and will not be called.\nDrag off pins to build functionality.
)

(event EventTick
  (params (DeltaSeconds :type Float%20%28single-precision%29))
  (|CallParentFunction DeltaSeconds) ; This node is disabled and will not be called.\nDrag off pins to build functionality.
)

(fn ConstructionScript
  (|CallParentFunction))